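; BP_ItemResource is an inventory item that adds a resource amount to a wallet when interacted with.
; On interaction it has the engaging actor's item inventory component show an interaction message for the item name.
; It then calls ModifyWalletMessage on the item inventory, using the item name as the wallet key and crediting its amount without marking it consumed.
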(event `self.ReceiveBeginPlay`
  (`parent.ReceiveBeginPlay`))

(event `/Game/Inventory/Blueprint/Utility/BPI_ItemInteraction.ItemInteract`
  (message `/Game/Inventory/Blueprint/Utility/BPI_PlayerInteraction.MakeItemInteraction` (`self.GetComponentByClass` (`self.EngageActor`) "/Game/Inventory/Blueprint/Master/BP_ItemInventoryComponent.BP_ItemInventoryComponent_C") (`self.ItemName`))
  (message `/Game/Inventory/Blueprint/Utility/BPI_ItemInventory.ModifyWallet` (`/Game/Inventory/Blueprint/Utility/BPL_ItemInventory.GetItemInventory`) (`self.ItemName`) (`self.Amount`) false))

(fn `UserConstructionScript`
  (`parent.UserConstructionScript`))