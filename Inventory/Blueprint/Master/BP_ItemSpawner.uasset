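; BP_ItemSpawner spawns item actors with a type, amount and name, placed relative to its SpawnTransform.
; Three events spawn in place, at a random horizontal offset within a radius, or at a distance along a direction.
; All call SpawnItemActor, which uses the given class if valid, otherwise looks up the actor class in DT_ItemParser by item type name.
; If that lookup finds no row, nothing spawns.
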(event `/Game/Inventory/Blueprint/Utility/BPI_ItemSpawn.SpawnItemInPlace`
  (params (SpawnTransform :type "Transform Structure") (Class :type "/Game/Inventory/Blueprint/Master/BP_ItemMaster Class Reference") (Type :type "/Game/Inventory/Enum/E_ItemType Enum" :default "NewEnumerator0") (Amount :type Integer) (ItemName :type Name))
  (`self.SpawnItemActor` Class SpawnTransform_Location SpawnTransform_Rotation SpawnTransform_Scale Amount Type ItemName))

(event `/Game/Inventory/Blueprint/Utility/BPI_ItemSpawn.SpawnItemInRange`
  (params (SpawnTransform :type "Transform Structure") (Class :type "/Game/Inventory/Blueprint/Master/BP_ItemMaster Class Reference") (Type :type "/Game/Inventory/Enum/E_ItemType Enum" :default "NewEnumerator0") (Amount :type Integer) (ItemName :type Name) (Radius :type "Float (double-precision)"))
  (bind (_returnvalue_x _returnvalue_y) (`KismetMathLibrary.BreakVector` (* Radius (`KismetMathLibrary.RandomUnitVector`))))
  (`self.SpawnItemActor` Class (+ SpawnTransform_Location (`KismetMathLibrary.MakeVector` _returnvalue_x _returnvalue_y)) SpawnTransform_Rotation SpawnTransform_Scale Amount Type ItemName))

(event `/Game/Inventory/Blueprint/Utility/BPI_ItemSpawn.SpawnItemInDirection`
  (params (SpawnTransform :type "Transform Structure") (Class :type "/Game/Inventory/Blueprint/Master/BP_ItemMaster Class Reference") (Type :type "/Game/Inventory/Enum/E_ItemType Enum" :default "NewEnumerator0") (Amount :type Integer) (ItemName :type Name) (Distance :type "Float (double-precision)") (Direction :type "Vector Structure"))
  (`self.SpawnItemActor` Class (+ SpawnTransform_Location (* Direction Distance)) SpawnTransform_Rotation SpawnTransform_Scale Amount Type ItemName))

(fn `SpawnItemActor`
  (params (Class :type "/Game/Inventory/Blueprint/Master/BP_ItemMaster Class Reference") (`Spawn Transform Location` :type "Vector Structure") (`Spawn Transform Rotation` :type "Rotator Structure") (`Spawn Transform Scale` :type "Vector Structure") (Amount :type Integer) (ItemType :type "/Game/Inventory/Enum/E_ItemType Enum" :default "NewEnumerator0") (ItemName :type Name))
  (locals (ActorClass :type "/Game/Inventory/Blueprint/Master/BP_ItemMaster Class Reference"))
  (if (`KismetSystemLibrary.IsValidClass` Class)
    (set `local.ActorClass` Class)
    (else
      (bind _returnvalue (`|GetDataTableRow` "/Game/Inventory/DataTables/DT_ItemParser.DT_ItemParser" (`KismetStringLibrary.Conv_StringToName` (`|GetEnumeratorNameAsString` ItemType)))
        (:`then`
          (set `local.ActorClass` (`.ItemActor_8_EE698B38404E0A3148EF7BB07F43BE8F` (break `/Game/Inventory/DataStruct/Master/ST_ItemParser` _returnvalue)))))))
  (`|SpawnActorFromClass` (`local.ActorClass`) (`KismetMathLibrary.MakeTransform` `Spawn Transform Location` `Spawn Transform Rotation` `Spawn Transform Scale`) "Undefined" "MultiplyWithRoot" null Amount ItemType ItemName null))

(fn `UserConstructionScript`)