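; Master actor for a world item that can be picked up into an inventory.
; On BeginPlay its ItemType selects a parser class from DT_ItemParser, which supplies the mesh and item data, with a random amount if unset.
; A trigger box scaled to the mesh toggles pickability and the name/amount widget, letting ItemInteract send the item to the inventory.
; Mesh physics stops on first hit, and destruction is a separate event.
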(event `self.ReceiveBeginPlay`
  (`self.Construct Item Data`))

(event `self.Box.OnComponentBeginOverlap`
  (params (OverlappedComponent :type "PrimitiveComponent Object Reference") (OtherActor :type "Actor Object Reference") (OtherComp :type "PrimitiveComponent Object Reference") (OtherBodyIndex :type Integer) (bFromSweep :type Boolean) (SweepResult :type "HitResult Structure (by ref)"))
  (set `self.IsPickable` true)
  (`SceneComponent.SetVisibility` (`self.Widget`) true false)
  (set `self.EngageActor` OtherActor))

(event `self.Box.OnComponentEndOverlap`
  (params (OverlappedComponent :type "PrimitiveComponent Object Reference") (OtherActor :type "Actor Object Reference") (OtherComp :type "PrimitiveComponent Object Reference") (OtherBodyIndex :type Integer))
  (set `self.IsPickable` false)
  (`SceneComponent.SetVisibility` (`self.Widget`) false false)
  (set `self.EngageActor` null))

(event `/Game/Inventory/Blueprint/Utility/BPI_ItemInteraction.ItemInteract`
  (`self.ModifyInventory`))

(event `self.StaticMesh.OnComponentHit`
  (params (HitComponent :type "PrimitiveComponent Object Reference") (OtherActor :type "Actor Object Reference") (OtherComp :type "PrimitiveComponent Object Reference") (NormalImpulse :type "Vector Structure") (Hit :type "HitResult Structure (by ref)"))
  (`PrimitiveComponent.SetSimulatePhysics` (`self.StaticMesh`) false))

(event `/Game/Inventory/Blueprint/Utility/BPI_ItemInteraction.ItemDestroy`
  (`self.K2_DestroyActor`))

(fn `Construct Item Data`
  (bind _returnvalue (`|GetDataTableRow` "/Game/Inventory/DataTables/DT_ItemParser.DT_ItemParser" (`KismetStringLibrary.Conv_StringToName` (`|GetEnumeratorNameAsString` (`self.ItemType`))))
    (:`then`
      (bind (_itemname _displayname _description _functionoverride _model) (`self.Init Item Parser` (`.AttributeParser_9_22D761644E223884ABD812A0AA351524` (break `/Game/Inventory/DataStruct/Master/ST_ItemParser` _returnvalue))))
      (set `self.ItemName` _itemname)
      (`StaticMeshComponent.SetStaticMesh` (`self.StaticMesh`) _model)
      (bind _returnvalue_2 (`|GenericCreateObject` "/Game/Inventory/DataStruct/Master/BP_CommonItemData.BP_CommonItemData_C" _displayname _description _itemname (`self.ItemType`) _functionoverride))
      (set `self.ItemData` _returnvalue_2)
      (if (== (`self.Amount`) 0)
        (set `self.Amount` (`KismetMathLibrary.RandomIntegerInRange` 1 50)))
      (`self.ScaleTriggerBox`)
      (bind _aswbp_item_interaction (cast `/Game/Inventory/UI/WBP_ItemInteraction` (`WidgetComponent.GetUserWidgetObject` (`self.Widget`))))
      (`/Game/Inventory/UI/WBP_ItemInteraction.SetDisplayText` _aswbp_item_interaction (`/Game/Inventory/DataStruct/Master/BP_CommonItemData.DisplayName` (`self.ItemData`)) (`self.Amount`)))))

(fn `Init Item Parser`
  (params (ParserClass :type "/Game/Inventory/Blueprint/Master/BP_ItemParserMaster Class Reference"))
  (returns (ItemName :type Name) (DisplayName :type Text) (Description :type Text) (FunctionOverride :type "/Game/Inventory/Blueprint/Master/BP_ItemParserMaster Class Reference") (Model :type "StaticMesh Object Reference"))
  (bind _returnvalue (`|GenericCreateObject` ParserClass))
  (set `self.ItemFunction` _returnvalue)
  (bind (_itemname _displayname _description _functionoverride _model) (`/Game/Inventory/Blueprint/Master/BP_ItemParserMaster.ReadAttributeFromDataTable` (`self.ItemFunction`) (`self.ItemName`)))
  (return _itemname _displayname _description _functionoverride _model))

(fn `ModifyInventory`
  (if (`self.IsPickable`)
    (message `/Game/Inventory/Blueprint/Utility/BPI_PlayerInteraction.MakeItemInteraction` (`self.GetComponentByClass` (`self.EngageActor`) "/Game/Inventory/Blueprint/Master/BP_ItemInventoryComponent.BP_ItemInventoryComponent_C") "default")
    (message `/Game/Inventory/Blueprint/Utility/BPI_ItemInventory.ModifyInventory` (`/Game/Inventory/Blueprint/Utility/BPL_ItemInventory.GetItemInventory`) (`self.ItemData`) (`self.Amount`) false)))

(fn `ScaleTriggerBox`
  (`SceneComponent.SetRelativeScale3D` (`self.Box`) (* (/ (`.BoxExtent` (`KismetSystemLibrary.GetComponentBounds` (`self.StaticMesh`))) (`.BoxExtent` (`KismetSystemLibrary.GetComponentBounds` (`self.Box`)))) (`KismetMathLibrary.Conv_DoubleToVector` 1.25))))

(fn `UserConstructionScript`)