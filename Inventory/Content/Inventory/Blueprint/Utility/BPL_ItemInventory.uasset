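; BPL_ItemInventory is a utility Blueprint library for the inventory system, providing player inventory lookup and UI input switching.
; It fetches BP_PlayerInventoryComponent from the player character, always using player index 0.
; Opening sets Game and UI input focused on a given widget and shows the cursor.
; Closing only hides the cursor, leaving the input mode unchanged; SetInventoryInputMode combines both paths behind a boolean.
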(fn `GetPlayerIntentoryComponent`
  (returns (ReturnValue :type "/Inventory/Inventory/Blueprint/InventoryComponent/BP_PlayerInventoryComponent Object Reference"))
  (return (`Actor.GetComponentByClass` (`GameplayStatics.GetPlayerCharacter` null) "/Inventory/Inventory/Blueprint/InventoryComponent/BP_PlayerInventoryComponent.BP_PlayerInventoryComponent_C")))

(fn `SetCloseUIInputMode`
  (params (__WorldContext :type "Object Object Reference"))
  (set `PlayerController.bShowMouseCursor` false (`GameplayStatics.GetPlayerController` null)))

(fn `SetInventoryInputMode`
  (params (bIsOpen :type Boolean) (InWidgetToFocus :type "Widget Object Reference"))
  (bind _returnvalue (`GameplayStatics.GetPlayerController` null))
  (if bIsOpen
    (`WidgetBlueprintLibrary.SetInputMode_GameAndUIEx` _returnvalue InWidgetToFocus "DoNotLock" false)
    (set `PlayerController.bShowMouseCursor` true _returnvalue)
    (else
      (set `PlayerController.bShowMouseCursor` false (`GameplayStatics.GetPlayerController` null)))))

(fn `SetOpenUIInputMode`
  (params (InWidgetToFocus :type "Widget Object Reference") (__WorldContext :type "Object Object Reference"))
  (bind _returnvalue (`GameplayStatics.GetPlayerController` null))
  (`WidgetBlueprintLibrary.SetInputMode_GameAndUIEx` _returnvalue InWidgetToFocus "DoNotLock" false)
  (set `PlayerController.bShowMouseCursor` true _returnvalue))