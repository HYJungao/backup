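; Inventory component that lets its owning character pick up world items and open or close the inventory through an item inventory controller.
; PickItem capsule-traces at the owner's location, stores the hit actor, sends it an interact message and rotates the owner to face it.
; MakeItemInteraction plays a montage looked up by name in a data table, disabling player input until completion, then tells the stored item to destroy itself.
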(event `self.ReceiveBeginPlay`)

(event `self.ReceiveTick`
  (params (DeltaSeconds :type "Float (single-precision)")))

(event `/Inventory/ItemMaster/Blueprint/BPI_PlayerInteraction.MakeItemInteraction`
  (params (AnimationName :type Name))
  (bind _returnvalue (`GameplayStatics.GetPlayerController` 0))
  (bind _returnvalue_2 (`GameplayStatics.GetPlayerCharacter` 0))
  (bind _returnvalue_3 (`|GetDataTableRow` "/Inventory/ItemMaster/DataTable/DT_InteractionAnimation.DT_InteractionAnimation" AnimationName)
    (:`then`
      (`|PlayMontage` (`Actor.GetComponentByClass` (`self.GetOwner`) "/Script/Engine.SkeletalMeshComponent") (`.Animation_5_37AC36CC46A0273101D597BF94AA0ED8` (break `/Inventory/ItemMaster/Struct/ST_InteractionAnimation` _returnvalue_3))
        (:`then`
          (`Actor.DisableInput` _returnvalue_2 _returnvalue))
        (:`OnCompleted`
          (`Actor.EnableInput` _returnvalue_2 _returnvalue)
          (message `/Inventory/ItemMaster/Blueprint/BPI_ItemInteraction.ItemDestroy` (`self.InteractActor`)))))))

(fn `CloseInventory`
  (`/Inventory/Inventory/Blueprint/BP_ItemInventoryController.CloseInventory` (`/Inventory/Inventory/Blueprint/BPL_ItemInventory.GetItemInventoryController`)))

(fn `PickItem`
  (bind _returnvalue (`self.GetOwner`))
  (bind _returnvalue_2 (`Actor.K2_GetActorLocation` (`self.GetOwner`)))
  (bind (_outhit _returnvalue_3) (`KismetSystemLibrary.CapsuleTraceSingleForObjects` :`Start` _returnvalue_2 :`End` _returnvalue_2 :`Radius` 40.0 :`HalfHeight` 100.0 :`ObjectTypes` (`|MakeArray` "ObjectTypeQuery8" :!type "EObjectTypeQuery Enum") :`DrawDebugType` "ForOneFrame"))
  (if _returnvalue_3
    (bind (_bblockinghit _binitialoverlap _time _distance _location _impactpoint _normal _impactnormal _physmat _hitactor) (`GameplayStatics.BreakHitResult` _outhit))
    (set `self.InteractActor` _hitactor)
    (message `/Inventory/ItemMaster/Blueprint/BPI_ItemInteraction.ItemInteract` _hitactor)
    (`Actor.K2_SetActorRotation` _returnvalue (`KismetMathLibrary.FindLookAtRotation` (`Actor.K2_GetActorLocation` _returnvalue) (`Actor.K2_GetActorLocation` _hitactor)) false)))

(fn `ShowInventory`
  (`/Inventory/Inventory/Blueprint/BP_ItemInventoryController.OpenInventory` (`/Inventory/Inventory/Blueprint/BPL_ItemInventory.GetItemInventoryController`)))