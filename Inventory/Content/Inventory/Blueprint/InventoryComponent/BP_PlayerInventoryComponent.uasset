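; Player inventory component that handles picking up world items and storing or consuming inventory entries.
; PickItem capsule-traces around the owner, messages the hit item and turns the owner toward it.
; MakeItemInteraction plays a data-table montage with input disabled, then tells the item to destroy itself.
; ModifyInventory stores or uses items, refreshes the inventory widget and applies the item's override function or its type's default on successful use.
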(event `/Inventory/ItemMaster/Blueprint/BPI_PlayerInteraction.MakeItemInteraction`
  (params (AnimationName :type Name))
  (bind _returnvalue (`GameplayStatics.GetPlayerController` 0))
  (bind _returnvalue_2 (`GameplayStatics.GetPlayerCharacter` 0))
  (bind _returnvalue_3 (`|GetDataTableRow` "/Inventory/ItemMaster/DataTable/DT_InteractionAnimation.DT_InteractionAnimation" AnimationName)
    (:`then`
      (`|PlayMontage` (`Actor.GetComponentByClass` (`self.GetOwner`) "/Script/Engine.SkeletalMeshComponent") (`.Animation_5_37AC36CC46A0273101D597BF94AA0ED8` (break `/Inventory/ItemMaster/Struct/ST_InteractionAnimation` _returnvalue_3))
        (:`then`
          (`Actor.DisableInput` _returnvalue_2 _returnvalue))
        (:`OnCompleted`
          (`Actor.EnableInput` _returnvalue_2 _returnvalue)
          (message `/Inventory/ItemMaster/Blueprint/BPI_ItemInteraction.ItemDestroy` (`self.InteractActor`)))))))

(fn `ModifyInventory`
  (params (Name :type "Name (by ref)") (Amount :type Integer) (Type :type "/Inventory/ItemMaster/Enum/E_ItemType Enum (by ref)" :default "NewEnumerator0") (DisplayName :type Text) (Description :type Text) (bConsumed :type Boolean) (FunctionOverride :type "/Inventory/ItemMaster/Blueprint/BP_ItemAttributeParserMaster Class Reference"))
  (returns (bSuccessful :type Boolean))
  (bind _bsuccessful (`self.ModifyInventoryCharacter` Name Amount Type DisplayName Description bConsumed FunctionOverride))
  (return _bsuccessful))

(fn `ModifyInventoryCharacter`
  (params (Name :type "Name (by ref)") (Amount :type Integer :default 1) (Type :type "/Inventory/ItemMaster/Enum/E_ItemType Enum (by ref)") (DisplayName :type Text) (Description :type Text) (bConsumed :type Boolean) (FunctionOverride :type "/Inventory/ItemMaster/Blueprint/BP_ItemAttributeParserMaster Class Reference"))
  (returns (bSuccessful :type Boolean))
  (bind _inventorywidget (`self.InventoryWidget`))
  (if bConsumed
    (bind (_bsuccessful _bfinalelement _itemfunctionoverride) (`self.Use Item` Name Amount Type))
    (`/Inventory/Inventory/UI/WBP_InventoryWidgetMaster.Refresh Open Inventory` _inventorywidget _bfinalelement)
    (if _bsuccessful
      (if (`KismetSystemLibrary.IsValidClass` _itemfunctionoverride)
        (bind _returnvalue (`|GenericCreateObject` _itemfunctionoverride))
        (`/Inventory/ItemMaster/Blueprint/BP_ItemAttributeParserMaster.ApplyItemFunction` _returnvalue)
        (else
          (`/Inventory/ItemMaster/Blueprint/BP_ItemAttributeParserMaster.ApplyItemFunction` (`.ItemFunction_50_FA7AE67F4E8F1B2E4CAA4BA565754140` (break `/Inventory/Inventory/Struct/ST_ItemInventoryEntry` (`BlueprintMapLibrary.Map_Find` (`self.Inventory`) Type)))))))
    (return _bsuccessful)
    (else
      (`self.Store Item` Name Amount Type DisplayName Description FunctionOverride)
      (`/Inventory/Inventory/UI/WBP_InventoryWidgetMaster.Refresh Open Inventory` _inventorywidget false)
      (return true))))

(fn `PickItem`
  (bind _returnvalue (`self.GetOwner`))
  (bind _returnvalue_2 (`Actor.K2_GetActorLocation` (`self.GetOwner`)))
  (bind (_outhit _returnvalue_3) (`KismetSystemLibrary.CapsuleTraceSingleForObjects` _returnvalue_2 _returnvalue_2 40.0 100.0 (`|MakeArray` "ObjectTypeQuery8" :!type "EObjectTypeQuery Enum")))
  (if _returnvalue_3
    (bind (_bblockinghit _binitialoverlap _time _distance _location _impactpoint _normal _impactnormal _physmat _hitactor) (`GameplayStatics.BreakHitResult` _outhit))
    (set `self.InteractActor` _hitactor)
    (message `/Inventory/ItemMaster/Blueprint/BPI_ItemInteraction.ItemInteract` _hitactor)
    (`Actor.K2_SetActorRotation` _returnvalue (`KismetMathLibrary.FindLookAtRotation` (`Actor.K2_GetActorLocation` _returnvalue) (`Actor.K2_GetActorLocation` _hitactor)) false)))