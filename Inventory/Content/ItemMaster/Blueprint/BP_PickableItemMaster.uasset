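; Base pickable item actor that can be added to an overlapping actor's inventory on interaction.
; A Box overlap shows a prompt widget, marks the item pickable and caches the actor; leaving reverses this.
; ItemInteract calls PickupItem, which sends an interaction message and the item data and amount to that actor's BP_InventoryComponentMaster.
; The mesh stops simulating physics on hit, and destruction is a separate ItemDestroy event.
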(event `self.Box.OnComponentBeginOverlap`
  (params (OverlappedComponent :type "PrimitiveComponent Object Reference") (OtherActor :type "Actor Object Reference") (OtherComp :type "PrimitiveComponent Object Reference") (OtherBodyIndex :type Integer) (bFromSweep :type Boolean) (SweepResult :type "HitResult Structure (by ref)"))
  (set `self.IsPickable` true)
  (`SceneComponent.SetVisibility` (`self.Widget`) true false)
  (set `self.EngageActor` OtherActor))

(event `self.Box.OnComponentEndOverlap`
  (params (OverlappedComponent :type "PrimitiveComponent Object Reference") (OtherActor :type "Actor Object Reference") (OtherComp :type "PrimitiveComponent Object Reference") (OtherBodyIndex :type Integer))
  (set `self.IsPickable` false)
  (`SceneComponent.SetVisibility` (`self.Widget`) false false)
  (set `self.EngageActor` null))

(event `/Inventory/ItemMaster/Blueprint/BPI_ItemInteraction.ItemInteract`
  (`self.PickupItem`))

(event `self.StaticMesh.OnComponentHit`
  (params (HitComponent :type "PrimitiveComponent Object Reference") (OtherActor :type "Actor Object Reference") (OtherComp :type "PrimitiveComponent Object Reference") (NormalImpulse :type "Vector Structure") (Hit :type "HitResult Structure (by ref)"))
  (`PrimitiveComponent.SetSimulatePhysics` (`self.StaticMesh`) false))

(event `/Inventory/ItemMaster/Blueprint/BPI_ItemInteraction.ItemDestroy`
  (`self.K2_DestroyActor`))

(fn `PickupItem`
  (bind _returnvalue (`self.GetComponentByClass` (`self.EngageActor`) "/Inventory/Inventory/Blueprint/InventoryComponent/BP_InventoryComponentMaster.BP_InventoryComponentMaster_C"))
  (if (`self.IsPickable`)
    (message `/Inventory/ItemMaster/Blueprint/BPI_PlayerInteraction.MakeItemInteraction` _returnvalue "default")
    (`/Inventory/Inventory/Blueprint/InventoryComponent/BP_InventoryComponentMaster.ModifyInventoryByReference` _returnvalue (`self.ItemData`) (`self.Amount`) false)))

(fn `UserConstructionScript`)