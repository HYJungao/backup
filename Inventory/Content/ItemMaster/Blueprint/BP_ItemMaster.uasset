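; Base world item actor that builds its data, mesh and interaction label at BeginPlay.
; ItemType selects a parser class from DT_ItemParser, which is instantiated to read the attributes for ItemName from a data table.
; The results set the static mesh and fill a BP_CommonItemData object, with a random Amount if unset.
; The trigger box scales slightly beyond the mesh bounds, and WBP_ItemInteraction shows name and amount.
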(event `self.ReceiveBeginPlay`
  (`self.Construct Item Data`))

(fn `Construct Item Data`
  (bind _returnvalue (`|GetDataTableRow` "/Inventory/ItemMaster/DataTable/DT_ItemParser.DT_ItemParser" (`KismetStringLibrary.Conv_StringToName` (`|GetEnumeratorNameAsString` (`self.ItemType`))))
    (:`then`
      (bind (_itemname _displayname _description _functionoverride _model) (`self.Init Item Parser` (`.AttributeParser_9_22D761644E223884ABD812A0AA351524` (break `/Inventory/ItemMaster/Struct/ST_ItemParser` _returnvalue))))
      (set `self.ItemName` _itemname)
      (`StaticMeshComponent.SetStaticMesh` (`self.StaticMesh`) _model)
      (bind _returnvalue_2 (`|GenericCreateObject` "/Inventory/Inventory/Struct/BP_CommonItemData.BP_CommonItemData_C" _displayname _description _itemname (`self.ItemType`) _functionoverride))
      (set `self.ItemData` _returnvalue_2)
      (if (== (`self.Amount`) 0)
        (set `self.Amount` (`KismetMathLibrary.RandomIntegerInRange` 1 50)))
      (`self.ScaleTriggerBox`)
      (bind _aswbp_item_interaction (cast `/Inventory/ItemMaster/UI/WBP_ItemInteraction` (`WidgetComponent.GetUserWidgetObject` (`self.Widget`))))
      (`/Inventory/ItemMaster/UI/WBP_ItemInteraction.SetDisplayText` _aswbp_item_interaction (`/Inventory/Inventory/Struct/BP_CommonItemData.DisplayName` (`self.ItemData`)) (`self.Amount`)))))

(fn `Init Item Parser`
  (params (ParserClass :type "/Inventory/ItemMaster/Blueprint/BP_ItemAttributeParserMaster Class Reference"))
  (returns (ItemName :type Name) (DisplayName :type Text) (Description :type Text) (FunctionOverride :type "/Inventory/ItemMaster/Blueprint/BP_ItemAttributeParserMaster Class Reference") (Model :type "StaticMesh Object Reference"))
  (bind _returnvalue (`|GenericCreateObject` ParserClass))
  (set `self.ItemAttribute` _returnvalue)
  (bind (_itemname _displayname _description _functionoverride _model) (`/Inventory/ItemMaster/Blueprint/BP_ItemAttributeParserMaster.ReadAttributeFromDataTable` (`self.ItemAttribute`) (`self.ItemName`)))
  (return _itemname _displayname _description _functionoverride _model))

(fn `ScaleTriggerBox`
  (`SceneComponent.SetRelativeScale3D` (`self.Box`) (* (/ (`.BoxExtent` (`KismetSystemLibrary.GetComponentBounds` (`self.StaticMesh`))) (`.BoxExtent` (`KismetSystemLibrary.GetComponentBounds` (`self.Box`)))) (`KismetMathLibrary.Conv_DoubleToVector` 1.25))))

(fn `UserConstructionScript`)