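; BP_ItemMoney is a money pickup item that adds currency to the wallet of the character who interacts with it.
; On ItemInteract, it checks that the engaged actor is valid and sends an interaction message to that actor's player item inventory component.
; It then messages the item inventory controller to modify that character's wallet, using the item name as the wallet key and its Amount as the value.
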(event `/Inventory/ItemMaster/Blueprint/BPI_ItemInteraction.ItemInteract`
  (bind _engageactor (`self.EngageActor`))
  (`/Engine/EditorBlueprintResources/StandardMacros.IsValid` _engageactor
    (:`Is Valid`
      (message `/Inventory/ItemMaster/Blueprint/BPI_PlayerInteraction.MakeItemInteraction` (`self.GetComponentByClass` _engageactor "/Inventory/Inventory/Blueprint/CharacterComponent/BP_PlayerItemInventoryComponent.BP_PlayerItemInventoryComponent_C") (`self.ItemName`))
      (message `/Inventory/Inventory/Blueprint/Utility/BPI_ItemInventory.ModifyCharacterWallet` (`/Inventory/Inventory/Blueprint/Utility/BPL_ItemInventory.GetItemInventoryController`) (`self.ItemName`) (`self.Amount`) false (`self.GetEngageActorName`)))))

(fn `UserConstructionScript`
  (`parent.UserConstructionScript`))