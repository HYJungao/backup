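; BP_ItemResource is a resource item that credits an amount of a named resource to the wallet of the actor interacting with it.
; On ItemInteract it looks up BP_InventoryComponentMaster on EngageActor, raises an interaction message for ItemName, then calls ModifyWallet with ItemName as the wallet key and Amount, flagged as not consumed.
; BeginPlay and construction only call the parent, and overlap and tick are disabled.
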(event `self.ReceiveBeginPlay`
  (`parent.ReceiveBeginPlay`))

(event `/Inventory/ItemMaster/Blueprint/BPI_ItemInteraction.ItemInteract`
  (bind _returnvalue (`self.GetComponentByClass` (`self.EngageActor`) "/Inventory/Inventory/Blueprint/InventoryComponent/BP_InventoryComponentMaster.BP_InventoryComponentMaster_C"))
  (message `/Inventory/ItemMaster/Blueprint/BPI_PlayerInteraction.MakeItemInteraction` _returnvalue (`self.ItemName`))
  (`/Inventory/Inventory/Blueprint/InventoryComponent/BP_InventoryComponentMaster.ModifyWallet` _returnvalue (`self.ItemName`) (`self.Amount`) false))

(fn `UserConstructionScript`
  (`parent.UserConstructionScript`))