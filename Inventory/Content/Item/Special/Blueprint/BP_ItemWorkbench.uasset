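; Interactable workbench item that opens a composition UI, apparently for crafting.
; On BeginPlay it creates and caches a WBP_WorkbenchMain widget, loads every DT_CompositionTable row into an array and passes that to the widget's RefreshView.
; ItemInteract adds the cached widget to the viewport and switches to inventory input mode with focus on it.
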(event `self.ReceiveBeginPlay`
  (`parent.ReceiveBeginPlay`)
  (`self.Init`))

(event `/Inventory/ItemMaster/Blueprint/BPI_ItemInteraction.ItemInteract`
  (bind _mainwidget (`self.MainWidget`))
  (`UserWidget.AddToViewport` _mainwidget 0)
  (`/Inventory/Inventory/Blueprint/Utility/BPL_ItemInventory.SetInventoryInputMode` true _mainwidget))

(fn `Get Composition Table`
  (bind _outrownames (`DataTableFunctionLibrary.GetDataTableRowNames` "/Inventory/Item/Special/DataTable/Workbench/DT_CompositionTable.DT_CompositionTable"))
  (for _array_element _outrownames
    (bind _returnvalue (`|GetDataTableRow` "/Inventory/Item/Special/DataTable/Workbench/DT_CompositionTable.DT_CompositionTable" _array_element)
      (:`then`
        (`KismetArrayLibrary.Array_Add` (`self.CompositionTable`) _returnvalue)))))

(fn `Init`
  (bind _returnvalue (`|CreateWidget` "/Inventory/Item/Special/UI/Workbench/WBP_WorkbenchMain.WBP_WorkbenchMain_C"))
  (set `self.MainWidget` _returnvalue)
  (`self.Get Composition Table`)
  (`/Inventory/Item/Special/UI/Workbench/WBP_WorkbenchMain.RefreshView` (`self.MainWidget`) (`self.CompositionTable`)))

(fn `UserConstructionScript`
  (`parent.UserConstructionScript`))